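; BP_Painting is an interactable painting actor that shows an information screen about the artwork.
; Overlapping its sphere shows a widget component, and leaving hides it.
; Interact uses a FlipFlop to alternately create a WP_Napeoleon viewport widget or remove it, playing a different sound at the actor each way.
; Helper functions fill that widget from the actor's Image, Title and Description variables.
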(event `self.ReceiveBeginPlay`)

(event `self.Sphere.OnComponentBeginOverlap`
  (params (OverlappedComponent :type "PrimitiveComponent Object Reference") (OtherActor :type "Actor Object Reference") (OtherComp :type "PrimitiveComponent Object Reference") (OtherBodyIndex :type Integer) (bFromSweep :type Boolean) (SweepResult :type "HitResult Structure (by ref)"))
  (`SceneComponent.SetVisibility` (`self.Widget`) true false))

(event `self.Sphere.OnComponentEndOverlap`
  (params (OverlappedComponent :type "PrimitiveComponent Object Reference") (OtherActor :type "Actor Object Reference") (OtherComp :type "PrimitiveComponent Object Reference") (OtherBodyIndex :type Integer))
  (`SceneComponent.SetVisibility` (`self.Widget`) false false))

(event `/Game/Blueprints/InteractInterface.Interact`
  (`/Engine/EditorBlueprintResources/StandardMacros.FlipFlop`
    (:`A`
      (bind _returnvalue (`|CreateWidget` "/Game/Blueprints/WP_Napeoleon.WP_Napeoleon_C"))
      (`Image.SetBrushFromTexture` (`/Game/Blueprints/WP_Napeoleon.Thumbnail` _returnvalue) (`self.Image`) false)
      (`TextBlock.SetText` (`/Game/Blueprints/WP_Napeoleon.DescriptionText` _returnvalue) (`KismetTextLibrary.Conv_StringToText` (`self.Description`)))
      (`TextBlock.SetText` (`/Game/Blueprints/WP_Napeoleon.Title` _returnvalue) (`KismetTextLibrary.Conv_StringToText` (`self.Title`)))
      (`UserWidget.AddToViewport` _returnvalue 0)
      (`GameplayStatics.PlaySoundAtLocation` "/Game/Blueprints/SFX/Tada_Sound.Tada_Sound" (`self.K2_GetActorLocation`) (struct) 1.0 1.0 0.0 null null null null))
    (:`B`
      (`Widget.RemoveFromParent` _returnvalue)
      (`GameplayStatics.PlaySoundAtLocation` "/Game/Blueprints/SFX/HM_Sound.HM_Sound" (`self.K2_GetActorLocation`) (struct) 1.0 1.0 0.0 null null null null))))

(fn `UserConstructionScript`)